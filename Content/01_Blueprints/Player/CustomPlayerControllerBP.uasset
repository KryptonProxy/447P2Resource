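; Player controller that owns the HUD and SpaceBux currency, and decides when the game is won or lost by that balance.
; BeginPlay creates the HUD and seeds starting funds, and the inventory input displays the player inventory through it.
; Every tick it checks the balance, showing a win or lose widget with UI-only input and pausing the game.
; ResourceMangement changes funds and refreshes the HUD money text, while AddSpaceBux and SubtractSpaceBux only change the value.
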(event `self.ReceiveBeginPlay`
  (bind _returnvalue (`|CreateWidget` "/Game/04_UI/HUD_UI.HUD_UI_C" (`GameplayStatics.GetPlayerController` 0)))
  (bind _output_get (set `self.HUDRef` _returnvalue))
  (`UserWidget.AddToViewport` _output_get 0)
  (set `self.SpaceBux` 160.0))

(event `self.ReceiveTick`
  (params (DeltaSeconds :type "Float (single-precision)"))
  (`self.Winner WInner Chicken Dinner`))

(event `EnhancedInput|/Game/05_Input/Actions/IA_Inventory`
  (params (ActionValue :type Boolean) (ElapsedSeconds :type "Float (double-precision)") (TriggeredSeconds :type "Float (double-precision)") (InputAction :type "InputAction Object Reference" :default "/Game/05_Input/Actions/IA_Inventory.IA_Inventory"))
  (:`Triggered`
    (`/Game/04_UI/HUD_UI.Display Player Inventory` (`self.HUDRef`))))

(event `Winner WInner Chicken Dinner`
  (bind _returnvalue (`GameplayStatics.GetPlayerController` 0))
  (bind _returnvalue_2 (`GameplayStatics.GetPlayerController` 0))
  (bind _lose (`self.Lose`))
  (bind _win (`self.Win`))
  (if (<= (`self.SpaceBux`) 0.0)
    (`WidgetBlueprintLibrary.SetInputMode_UIOnlyEx` _returnvalue (`self.Lose`))
    (`/Engine/EditorBlueprintResources/StandardMacros.IsValid` _lose
      (:`Is Valid`
        (if (`Widget.IsInViewport` _lose)
          (`GameplayStatics.SetGamePaused` true :!label _label)))
      (:`Is Not Valid`
        (set `PlayerController.bShowMouseCursor` true _returnvalue)
        (bind _returnvalue_3 (`|CreateWidget` "/Game/04_UI/Lose_UI.Lose_UI_C" _returnvalue))
        (bind _output_get (set `self.Lose` _returnvalue_3))
        (`UserWidget.AddToViewport` _output_get 0)
        (goto _label)))
    (elif (>= (`self.SpaceBux`) 3000.0)
      (`WidgetBlueprintLibrary.SetInputMode_UIOnlyEx` _returnvalue_2 (`self.Win`))
      (`/Engine/EditorBlueprintResources/StandardMacros.IsValid` _win
        (:`Is Valid`
          (if (`Widget.IsInViewport` _win)
            (`GameplayStatics.SetGamePaused` true :!label _label_2)))
        (:`Is Not Valid`
          (set `PlayerController.bShowMouseCursor` true _returnvalue_2)
          (bind _returnvalue_4 (`|CreateWidget` "/Game/04_UI/Win_UI.Win_UI_C" _returnvalue_2))
          (bind _output_get_2 (set `self.Win` _returnvalue_4))
          (`UserWidget.AddToViewport` _output_get_2 0)
          (goto _label_2))))))

(event `AddSpaceBux`
  (params (B :type "Float (double-precision)"))
  (set `self.SpaceBux` (+ (`self.SpaceBux`) B)))

(event `SubtractSpaceBux`
  (params (B :type "Float (double-precision)"))
  (set `self.SpaceBux` (- (`self.SpaceBux`) B)))

(fn `ResourceMangement`
  (params (Amount :type "Float (double-precision)"))
  (bind _output_get (set `self.SpaceBux` (+ Amount (`self.SpaceBux`))))
  (`TextBlock.SetText` (`/Game/04_UI/HUD_UI.MoneyAmountText` (`self.HUDRef`)) (`KismetTextLibrary.Conv_DoubleToText` _output_get "HalfToEven")))

(fn `UserConstructionScript`)